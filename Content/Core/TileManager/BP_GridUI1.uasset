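; Grid UI actor for the tile system that draws movement paths, a hover marker, a target marker and tile markers.
; Paths are spline points covered with spline mesh segments cut at tile-size intervals, each tinted through a dynamic material with fade at both ends.
; Tile markers by type, such as move and range, map to meshes batched in per-mesh hierarchical instanced components, created on demand and cached for clearing.
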(event Custom|SetHoverVisibility
  (params (bNewVisibility :type Boolean))
  (Rendering|SetVisibility (Variables|Default|GetHoverMarker) bNewVisibility true))

(event Custom|DisplayPath
  (params (SplineMeshVectors :type Array%20of%20Vectors) (Color :type Linear%20Color%20Structure :default "(R=1.000000,G=1.000000,B=1.000000,A=1.000000)") (bClearOldPath :type Boolean))
  (Spline|SetSplinePoints (Variables|Default|GetSpline) SplineMeshVectors "World" true)
  (Utilities|UpdateSplinePointTypes (Variables|Default|GetSpline) (Variables|Default|GetSplineType))
  (CallFunction|DisplaySplineMeshPath bClearOldPath Color))

(event Custom|DisplayTargetMarker
  (params (TargetLocation :type Vector) (bNewVisibility :type Boolean))
  (Transformation|SetWorldLocation (Variables|Default|GetTargetMarker) TargetLocation false false)
  (Rendering|SetVisibility (Variables|Default|GetTargetMarker) bNewVisibility true)
  (if bNewVisibility
    _))

(event Custom|DisplayHover
  (params (HoverLocation :type Vector%20%28by%20ref%29))
  (Transformation|SetWorldLocation (Variables|Default|GetHoverMarker) HoverLocation false false))

(fn ConstructionScript)

(fn DisplaySplineMeshPath
  (params (bDestroyOldSplineMeshes :type Boolean) (Color :type Linear%20Color%20Structure))
  (bind _tilescalefactor (Variables|Default|GetTileScaleFactor))
  (bind _spline (Variables|Default|GetSpline))
  (if bDestroyOldSplineMeshes
    (CallFunction|ClearSplinePath))
  (LocalVariables|SetLocalTileSize (* (Variables|Default|GetTileSize) (Variables|Default|GetTileScaleFactor)))
  (LocalVariables|SetLastSplineIndex (.ReturnValue (Math|Float|Division(WholeandRemainder) (Spline|GetSplineLength (Variables|Default|GetSpline)) (+ (LocalVariables|GetLocalTileSize) 0.1))))
  (for _index (range 0 (.ReturnValue (Math|Float|Division(WholeandRemainder) (Spline|GetSplineLength (Variables|Default|GetSpline)) (+ (LocalVariables|GetLocalTileSize) 0.1)))) ; Add spline meshes from start to end of the spline
    (LocalVariables|SetLocalIndex _index)
    (bind _returnvalue (AddComponent|AddSplineMeshComponent true (Math|Transform|MakeTransform "0, 0, 0" "0, 0, 0" (Math|Conversions|ToVector(Float) (Variables|Default|GetTileScaleFactor)))))
    (Class|PrimitiveComponent|SetRenderinDepthPass _returnvalue true)
    (Transformation|SetMobility _returnvalue "Movable")
    (Components|StaticMesh|SetStaticMesh _returnvalue (Variables|Default|GetSplineAppearance))
    (Utilities|Array|Add (Variables|Default|GetSplineMeshes) _returnvalue)
    (SplineMesh|SetStartandEnd _returnvalue (/ (+ (Spline|GetLocationatDistanceAlongSpline _spline (* _index (LocalVariables|GetLocalTileSize)) "World") (Math|Vector|MakeVector 0.0 0.0 (Variables|Default|GetSplineHeight))) _tilescalefactor) "0, 0, 0" (/ (+ (Spline|GetLocationatDistanceAlongSpline _spline (+ (* _index (LocalVariables|GetLocalTileSize)) (LocalVariables|GetLocalTileSize)) "World") (Math|Vector|MakeVector 0.0 0.0 (Variables|Default|GetSplineHeight))) _tilescalefactor) "0, 0, 0" true :!class /Script/Engine.SplineMeshComponent)
    (bind _returnvalue_2 (Rendering|Material|CreateDynamicMaterialInstance _returnvalue 0 (Rendering|Material|GetMaterial _returnvalue 0) "None" :!class /Script/Engine.PrimitiveComponent))
    (Rendering|Material|SetVectorParameterValue _returnvalue_2 "Color" Color :!class /Script/Engine.MaterialInstanceDynamic)
    (Rendering|Material|SetScalarParameterValue _returnvalue_2 "Fade" (Math|Float|SelectFloat (Math|Float|SelectFloat -0.05 0.05 (== (LocalVariables|GetLocalIndex) 0)) 0.0 (or (== (LocalVariables|GetLocalIndex) 0) (== (LocalVariables|GetLocalIndex) (LocalVariables|GetLastSplineIndex)))) :!class /Script/Engine.MaterialInstanceDynamic))
  (return))

(fn ClearSplinePath
  (for _array_element (Variables|Default|GetSplineMeshes)
    (Components|DestroyComponent _array_element))
  (Utilities|Array|Clear (Variables|Default|GetSplineMeshes)))

(fn ClearAllTileMarkers
  (for _array_element (Utilities|Array|MakeArray "NewEnumerator0" "NewEnumerator1" "NewEnumerator2" "NewEnumerator3" "NewEnumerator4")
    (CallFunction|ClearMeshInstances (CallFunction|GetDefaultMarkerMesh _array_element)))
  (CallFunction|DisplayTargetMarker "0, 0, 0" false))

(fn ClearMeshInstances
  (params (StaticMesh :type Static%20Mesh%20Object%20Reference%20%28by%20ref%29))
  (bind _meshinstances (Variables|Default|GetMeshInstances))
  (bind (_value _returnvalue) (Utilities|Map|Find _meshinstances StaticMesh))
  (if _returnvalue
    (Components|InstancedStaticMesh|ClearInstances _value)
    (else
      (return))))

(fn SpawnTileMarkers
  (params (TileLocations :type Array%20of%20Vectors) (MarkerType :type ETileMarkerType%20Enum :default "NewEnumerator0"))
  (CallFunction|SpawnMeshInstancesatLocations (CallFunction|GetDefaultMarkerMesh MarkerType) TileLocations 0.0 true))

(fn GetDefaultMarkerMesh
  (params (MarkerType :type ETileMarkerType%20Enum :default "NewEnumerator0"))
  (return (Utilities|Select :Index MarkerType :NewEnumerator0 "/Game/TBS/StaticMeshes/Tiles/TilePlane_Move.TilePlane_Move" :NewEnumerator1 "/Game/TBS/StaticMeshes/Tiles/TilePlane_Range.TilePlane_Range" :NewEnumerator2 0 :NewEnumerator3 0 :NewEnumerator4 0)))

(fn SpawnMeshInstancesatLocations
  (params (MarkerMesh :type Static%20Mesh%20Object%20Reference%20%28by%20ref%29) (TileLocations :type Array%20of%20Vectors) (Offset :type Float%20%28double-precision%29) (bScaleToTileSize :type Boolean))
  (for _array_element TileLocations
    (Utilities|Array|Add (LocalVariables|GetLocal) (Math|Transform|MakeTransform (Math|Vector|MakeVector (.x _array_element) (.y _array_element) (.z _array_element)) "0, 0, 0" "1.000000,1.000000,1.000000")))
  (bind _meshhism (CallFunction|GetorAddMeshHism MarkerMesh))
  (Components|InstancedStaticMesh|AddInstances _meshhism (LocalVariables|GetLocal) false true))

(fn GetorAddMeshHism
  (params (StaticMesh :type Static%20Mesh%20Object%20Reference%20%28by%20ref%29))
  (bind _meshinstances (Variables|Default|GetMeshInstances))
  (bind (_value _returnvalue) (Utilities|Map|Find _meshinstances StaticMesh))
  (if _returnvalue
    (return _value)
    (else
      (bind _returnvalue_2 (Game|AddComponentbyClass "/Script/Engine.HierarchicalInstancedStaticMeshComponent" false))
      (Collision|SetCollisionEnabled _returnvalue_2 "NoCollision")
      (Rendering|Material|SetMaterial _returnvalue_2 0 0)
      (Components|StaticMesh|SetStaticMesh _returnvalue_2 StaticMesh)
      (Utilities|Map|Add (Variables|Default|GetMeshInstances) StaticMesh _returnvalue_2)
      (return _value))))

(fn ClearTileMarkers
  (params (MarkerType :type ETileMarkerType%20Enum :default "NewEnumerator0"))
  (CallFunction|ClearMeshInstances (CallFunction|GetDefaultMarkerMesh MarkerType)))

(fn SpawnMeshInstancesatTransforms
  (params (StaticMesh :type Static%20Mesh%20Object%20Reference%20%28by%20ref%29) (Transforms :type Array%20of%20Transforms))
  (bind _meshhism (CallFunction|GetorAddMeshHism StaticMesh))
  (for _array_element Transforms
    (Components|InstancedStaticMesh|AddInstance _meshhism _array_element true)))